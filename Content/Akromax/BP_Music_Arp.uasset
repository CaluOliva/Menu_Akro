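; BP_Music_Arp is an actor that moves its EsferaMelodi component along a spline, apparently as part of a musical arpeggio element.
; Each Tick adds Velocidad times delta time to Distancia and samples the spline's location and rotation there, keeping the component's scale.
; The world-space sample is applied as a relative transform.
; When IsLooping is set, Distancia resets to zero after passing the spline's end.
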(event EventBeginPlay)

(event Collision|EventActorBeginOverlap
  (params (OtherActor :type Actor%20Object%20Reference)))

(event EventTick
  (params (DeltaSeconds :type Float%20%28single-precision%29))
  (Variables|Default|SetDistancia (+ (* DeltaSeconds (Variables|Default|GetVelocidad)) (Variables|Default|GetDistancia)))
  (Transformation|SetRelativeTransform (Variables|Default|GetEsfera_melodi) (Math|Transform|MakeTransform (.location (Spline|GetTransformatDistanceAlongSpline (Variables|Default|GetSpline) (Variables|Default|GetDistancia) "World" false)) (.rotation (Spline|GetTransformatDistanceAlongSpline (Variables|Default|GetSpline) (Variables|Default|GetDistancia) "World" false)) (Variables|/Script/Engine.SceneComponent|GetRelativeScale3D (Variables|Default|GetEsfera_melodi))) false false)
  (if (Variables|Default|GetIs%20Looping)
    (if (> (Variables|Default|GetDistancia) (Spline|GetSplineLength (Variables|Default|GetSpline)))
      (Variables|Default|SetDistancia 0.0))))

(fn ConstructionScript)